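; BP_TestEnemy is a test enemy pawn that patrols a path and chases the player on sight.
; Tick switches between Patrol, walking the BP_Path spline points in a loop via AI MoveTo, and Chase, following the target until it passes a give-up distance.
; Detection uses a sphere overlap filtered to BP_TPSPlayer within a field-of-view angle.
; Each tick also slerps rotation toward the velocity direction for smooth turning.
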(event Custom|AIPatrol
  (if (not (Variables|Default|GetbCanNotAIPatrol))
    (Variables|Default|SetbCanNotAIPatrol true)
    (AI|AIMoveTo self (Spline|GetLocationatSplinePoint (Variables|Default|GetSpline) (Variables|Default|GetCurrentIndex) "World") 0 5.0 false
      (:OnSuccess
        (bind _result (Math|Integer|IncrementInt (Variables|Default|GetCurrentIndex))
          (:%20%20
            (if (>= _result (Spline|GetNumberOfSplinePoints (Variables|Default|GetSpline)))
              (Variables|Default|SetCurrentIndex 0))
            (Variables|Default|SetbCanNotAIPatrol false)
            (CallFunction|AIPatrol)))))))

(event Custom|FindPlayer
  (bind _outactors (Collision|SphereOverlapActors (Transformation|GetActorLocation) 3e+02 (Utilities|Array|MakeArray "ObjectTypeQuery3") 0 (Utilities|Array|MakeArray self)))
  (bind _array_element (Utilities|Array|ForEachLoopwithBreak _outactors :!label _label)
    (:LoopBody
      (bind _asbp_tpsplayer (Utilities|Casting|CastToBP_TPSPlayer _array_element))
      (bind _returnvalue (Class|TestEnemy|GetFovAngle (Transformation|GetActorForwardVector) (- (Transformation|GetActorLocation _asbp_tpsplayer) (Transformation|GetActorLocation))))
      (Development|PrintString (Utilities|String|ToString(Float) _returnvalue))
      (if (<= _returnvalue (Variables|Default|GetFovAngle))
        (Variables|Default|SetChaseTarget _asbp_tpsplayer)
        (Variables|Default|SetState "NewEnumerator1")
        (goto _label Break)))))

(event Custom|AIChase
  (AI|AIMoveTo self "0, 0, 0" (Variables|Default|GetChaseTarget) 5.0 false))

(event Custom|CheckGiveup
  (if (> (Transformation|GetDistanceTo (Variables|Default|GetChaseTarget)) (Variables|Default|GetGiveupDistance))
    (Variables|Default|SetbCanNotAIPatrol false)
    (Variables|Default|SetState "NewEnumerator0")))

(event EventBeginPlay
  (Variables|Default|SetState "NewEnumerator0")
  (bind _returnvalue (Actor|GetActorOfClass "/Game/TPS/Blueprints/BP_Path.BP_Path_C"))
  (Variables|Default|SetSpline (Variables|/Game/TPS/Blueprints/BP_Path.BP_Path_C|GetSpline _returnvalue))
  (Variables|Default|SetCurrentIndex 0))

(event Collision|EventActorBeginOverlap
  (params (OtherActor :type Actor%20Object%20Reference)))

(event EventTick
  (params (DeltaSeconds :type Float%20%28single-precision%29))
  (Utilities|FlowControl|Sequence
    (:then_0
      (switch Utilities|FlowControl|Switch|SwitchonETestEnemyState (Variables|Default|GetState)
        (:NewEnumerator0
          (CallFunction|AIPatrol)
          (CallFunction|FindPlayer))
        (:NewEnumerator1
          (CallFunction|AIChase)
          (CallFunction|CheckGiveup))))
    (:then_1
      (Transformation|SetActorRotation (Class|KismetMathLibrary|QuatRotator (Class|KismetMathLibrary|QuatSlerp (Math|Conversions|ToQuaternion(Rotator) (Transformation|GetActorRotation)) (Math|Conversions|ToQuaternion(Rotator) (Math|Rotator|MakeRotfromXZ (Transformation|GetVelocity) (Transformation|GetActorUpVector))) 0.1))))))

(fn ConstructionScript)